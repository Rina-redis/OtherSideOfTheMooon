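; Pistol weapon Blueprint that extends a parent weapon class and fires projectile actors with effectively unlimited ammo.
; BeginPlay runs the parent logic, then sets CurrentAmmo to the maximum integer.
; Fire spawns a BP_ShotGun_Bullet at the Box component's "Ammo" socket, aimed along the player 0 camera rotation.
; The rotated forward offset on the spawn location is zero, so bullets appear exactly at the socket.
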(event EventBeginPlay
  (|CallParentFunction)
  (Variables|Default|SetCurrentAmmo 2147483647))

(event Collision|EventActorBeginOverlap
  (params (OtherActor :type Actor%20Object%20Reference))
  (|CallParentFunction OtherActor) ; This node is disabled and will not be called.\nDrag off pins to build functionality.
)

(event EventTick
  (params (DeltaSeconds :type Float%20%28single-precision%29))
  (|CallParentFunction DeltaSeconds) ; This node is disabled and will not be called.\nDrag off pins to build functionality.
)

(event EventFire
  (bind _returnvalue (Game|GetPlayerCameraManager 0))
  (bind _returnvalue_2 (Camera|GetCameraRotation _returnvalue))
  (Game|SpawnActorfromClass "/Game/Weapons/Bullets/BP_ShotGun_Bullet.BP_ShotGun_Bullet_C" (Math|Transform|MakeTransform (+ (Transformation|GetSocketLocation (Variables|Default|GetBox) "Ammo") (Math|Vector|RotateVector "0, 0, 0" _returnvalue_2)) _returnvalue_2) "Undefined" "MultiplyWithRoot" 0 0))

(fn ConstructionScript
  (|CallParentFunction))